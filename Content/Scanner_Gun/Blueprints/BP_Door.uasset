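; BP_Door is a door in the Scanner_Gun content that starts closed to pawns and can be opened through an OpenDoor event.
; While it is closed, a Character entering its Box trigger gets a W_Game widget on screen, removed again when a Character leaves.
; OpenDoor sets the Cube to ignore the Pawn channel, flags the door open and clears the widget, making it passable without any movement.
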(event `Open Door`
  (`PrimitiveComponent.SetCollisionResponseToChannel` (`self.Cube`) "ECC_Pawn" "ECR_Ignore")
  (set `self.Open?` true)
  (`/Engine/EditorBlueprintResources/StandardMacros.IsValid` (stale `self.Box.OnComponentBeginOverlap` _returnvalue)
    (:`Is Valid`
      (`Widget.RemoveFromParent` (stale `self.Box.OnComponentBeginOverlap` _returnvalue)))))

(event `self.Box.OnComponentBeginOverlap`
  (params (OverlappedComponent :type "PrimitiveComponent Object Reference") (OtherActor :type "Actor Object Reference") (OtherComp :type "PrimitiveComponent Object Reference") (OtherBodyIndex :type Integer) (bFromSweep :type Boolean) (SweepResult :type "HitResult Structure (by ref)"))
  (cast `Character` OtherActor)
  (if (not (`self.Open?`))
    (bind _returnvalue (`|CreateWidget` "/Game/Scanner_Gun/widget/W_Game.W_Game_C"))
    (`UserWidget.AddToViewport` _returnvalue 0)))

(event `self.Box.OnComponentEndOverlap`
  (params (OverlappedComponent :type "PrimitiveComponent Object Reference") (OtherActor :type "Actor Object Reference") (OtherComp :type "PrimitiveComponent Object Reference") (OtherBodyIndex :type Integer))
  (cast `Character` OtherActor)
  (`/Engine/EditorBlueprintResources/StandardMacros.IsValid` (stale `self.Box.OnComponentBeginOverlap` _returnvalue)
    (:`Is Valid`
      (`Widget.RemoveFromParent` (stale `self.Box.OnComponentBeginOverlap` _returnvalue)))))

(fn `UserConstructionScript`)