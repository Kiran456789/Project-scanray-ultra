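; Scene-level manager that renders the Scanner Gun's laser dots as colored hierarchical instanced meshes in yellow, green, blue and red.
; Each color has a permanent component and a buffer component created on demand to receive new points.
; Past 2000 instances, BufferTransfer is called to copy points in 500-step chunks into the permanent component.
; The buffer reference is then cleared without destroying its component, so the next point creates another.
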(event `SpawnBufferYellowPoint`
  (params (`Instance Transform Location` :type "Vector Structure") (`Instance Transform Rotation` :type "Rotator Structure"))
  (bind _bufferyellow (`self.bufferYellow`))
  ;[1 0.7986 0.307 1 52] Buffer Point
  ;;[1 1 1] You can duplicate this code to add your new color
  (`/Engine/EditorBlueprintResources/StandardMacros.IsValid` (`self.bufferYellow`)
    (:`Is Valid`
      _)
    (:`Is Not Valid`
      (bind _returnvalue (`AddComponent|NODE_AddPointHierarchicalInstanced-4`))
      (`PrimitiveComponent.SetMaterial` _returnvalue 0 "/Game/Scanner_Gun/Materials/M_LaserYellowPoint.M_LaserYellowPoint")
      (set `self.bufferYellow` _returnvalue)))
  (`|ExecutionSequence`
    (:`then_0`
      (`InstancedStaticMeshComponent.SetCullDistances` _bufferyellow 0 0)
      (`InstancedStaticMeshComponent.AddInstance` _bufferyellow (`KismetMathLibrary.MakeTransform` `Instance Transform Location` `Instance Transform Rotation` (`self.Scale`)) false))
    (:`then_1`
      (if (> (`InstancedStaticMeshComponent.GetInstanceCount` (`self.bufferYellow`)) 2000)
        (`|ExecutionSequence`
          (:`then_0`
            (`self.Buffer Transfer` (`self.bufferYellow`)))
          (:`then_1`
            (set `self.bufferYellow` null)))))))

(event `Spawn Yellow Dot`
  (params (`Instance Transform Location` :type "Vector Structure") (`Instance Transform Rotation` :type "Rotator Structure"))
  (bind _yellowpoint (`self.YellowPoint`))
  ;[0.4683 1 0.4077 1 52] Permanent Point
  ;;[1 1 1] color
  ;;;[1 1 1] You can duplicate this code to add your new color
  (`InstancedStaticMeshComponent.SetCullDistances` _yellowpoint 0 0)
  (`InstancedStaticMeshComponent.AddInstance` _yellowpoint (`KismetMathLibrary.MakeTransform` `Instance Transform Location` `Instance Transform Rotation` (`self.Scale`)) false))

(event `Spawn Green Dot`
  (params (`Instance Transform Location` :type "Vector Structure") (`Instance Transform Rotation` :type "Rotator Structure"))
  (bind _greenpoint (`self.GreenPoint`))
  ;[0.4683 1 0.4077 1 52] Permanent Point
  ;;[1 1 1] color
  (`InstancedStaticMeshComponent.SetCullDistances` _greenpoint 0 0)
  (`InstancedStaticMeshComponent.AddInstance` _greenpoint (`KismetMathLibrary.MakeTransform` `Instance Transform Location` `Instance Transform Rotation` (`self.Scale`)) false))

(event `SpawnBufferGreenPoint`
  (params (`Instance Transform Location` :type "Vector Structure") (`Instance Transform Rotation` :type "Rotator Structure"))
  (bind _buffergreen (`self.bufferGreen`))
  ;[1 0.7986 0.307 1 52] Buffer Point
  (`/Engine/EditorBlueprintResources/StandardMacros.IsValid` (`self.bufferGreen`)
    (:`Is Valid`
      _)
    (:`Is Not Valid`
      (bind _returnvalue (`AddComponent|NODE_AddPointHierarchicalInstanced-5`))
      (`PrimitiveComponent.SetMaterial` _returnvalue 0 "/Game/Scanner_Gun/Materials/M_LaserGreenPoint.M_LaserGreenPoint")
      (set `self.bufferGreen` _returnvalue)))
  (`|ExecutionSequence`
    (:`then_0`
      (`InstancedStaticMeshComponent.SetCullDistances` _buffergreen 0 0)
      (`InstancedStaticMeshComponent.AddInstance` _buffergreen (`KismetMathLibrary.MakeTransform` `Instance Transform Location` `Instance Transform Rotation` (`self.Scale`)) false))
    (:`then_1`
      (if (> (`InstancedStaticMeshComponent.GetInstanceCount` (`self.bufferGreen`)) 2000)
        (`|ExecutionSequence`
          (:`then_0`
            (`self.Buffer Transfer` (`self.bufferGreen`) 1))
          (:`then_1`
            (set `self.bufferGreen` null)))))))

(event `Spawn Red Dot`
  (params (`Instance Transform Location` :type "Vector Structure") (`Instance Transform Rotation` :type "Rotator Structure"))
  (bind _redpoint (`self.RedPoint`))
  ;[0.4683 1 0.4077 1 52] Permanent Point
  ;;[1 1 1] color
  (`InstancedStaticMeshComponent.SetCullDistances` _redpoint 0 0)
  (`InstancedStaticMeshComponent.AddInstance` _redpoint (`KismetMathLibrary.MakeTransform` `Instance Transform Location` `Instance Transform Rotation` (`self.Scale`)) false))

(event `Spawn Blue Dot`
  (params (`Instance Transform Location` :type "Vector Structure") (`Instance Transform Rotation` :type "Rotator Structure"))
  (bind _bluepoint (`self.BluePoint`))
  ;[0.4683 1 0.4077 1 52] Permanent Point
  ;;[1 1 1] color
  (`InstancedStaticMeshComponent.SetCullDistances` _bluepoint 0 0)
  (`InstancedStaticMeshComponent.AddInstance` _bluepoint (`KismetMathLibrary.MakeTransform` `Instance Transform Location` `Instance Transform Rotation` (`self.Scale`)) false))

(event `SpawnBufferBluePoint`
  (params (`Instance Transform Location` :type "Vector Structure") (`Instance Transform Rotation` :type "Rotator Structure"))
  (bind _bufferblue (`self.bufferBlue`))
  ;[1 0.7986 0.307 1 52] Buffer Point
  (`/Engine/EditorBlueprintResources/StandardMacros.IsValid` (`self.bufferBlue`)
    (:`Is Valid`
      _)
    (:`Is Not Valid`
      (bind _returnvalue (`AddComponent|NODE_AddPointHierarchicalInstanced-6`))
      (`PrimitiveComponent.SetMaterial` _returnvalue 0 "/Game/Scanner_Gun/Materials/M_LaserBluePoint.M_LaserBluePoint")
      (set `self.bufferBlue` _returnvalue)))
  (`|ExecutionSequence`
    (:`then_0`
      (`InstancedStaticMeshComponent.SetCullDistances` _bufferblue 0 0)
      (`InstancedStaticMeshComponent.AddInstance` _bufferblue (`KismetMathLibrary.MakeTransform` `Instance Transform Location` `Instance Transform Rotation` (`self.Scale`)) false))
    (:`then_1`
      (if (> (`InstancedStaticMeshComponent.GetInstanceCount` (`self.bufferBlue`)) 2000)
        (`|ExecutionSequence`
          (:`then_0`
            (`self.Buffer Transfer` (`self.bufferBlue`) 2))
          (:`then_1`
            (set `self.bufferBlue` null)))))))

(event `SpawnBufferRedPoint`
  (params (`Instance Transform Location` :type "Vector Structure") (`Instance Transform Rotation` :type "Rotator Structure"))
  (bind _bufferred (`self.bufferRed`))
  ;[1 0.7986 0.307 1 52] Buffer Point
  (`/Engine/EditorBlueprintResources/StandardMacros.IsValid` (`self.bufferRed`)
    (:`Is Valid`
      _)
    (:`Is Not Valid`
      (bind _returnvalue (`AddComponent|NODE_AddPointHierarchicalInstanced-7`))
      (`PrimitiveComponent.SetMaterial` _returnvalue 0 "/Game/Scanner_Gun/Materials/M_LaserRedPoint.M_LaserRedPoint")
      (set `self.bufferRed` _returnvalue)))
  (`|ExecutionSequence`
    (:`then_0`
      (`InstancedStaticMeshComponent.SetCullDistances` _bufferred 0 0)
      (`InstancedStaticMeshComponent.AddInstance` _bufferred (`KismetMathLibrary.MakeTransform` `Instance Transform Location` `Instance Transform Rotation` (`self.Scale`)) false))
    (:`then_1`
      (if (> (`InstancedStaticMeshComponent.GetInstanceCount` (`self.bufferRed`)) 2000)
        (`|ExecutionSequence`
          (:`then_0`
            (`self.Buffer Transfer` (`self.bufferRed`) 3))
          (:`then_1`
            (set `self.bufferRed` null)))))))

(fn `Buffer Transfer`
  (params (buffer :type "InstancedStaticMeshComponent Object Reference") (`color selection` :type Integer))
  (bind _step (`self.Step`))
  (bind _returnvalue (- (`InstancedStaticMeshComponent.GetInstanceCount` buffer) 1))
  (while (>= _step _returnvalue)
    (if (<= _step _returnvalue)
      (for _index (range (- _step 500) (+ _step 1))
        (switch `int` `color selection`
          (:`Default`
            (bind _outinstancetransform (`InstancedStaticMeshComponent.GetInstanceTransform` buffer _index false))
            (`self.Spawn Yellow Dot` (.location _outinstancetransform) (.rotation _outinstancetransform) :!label _label))
          (:`0`
            (goto _label))
          (:`1`
            (`self.Spawn Green Dot` (.location _outinstancetransform) (.rotation _outinstancetransform)))
          (:`2`
            (`self.Spawn Blue Dot` (.location _outinstancetransform) (.rotation _outinstancetransform)))
          (:`3`
            (`self.Spawn Red Dot` (.location _outinstancetransform) (.rotation _outinstancetransform)))))
      (set `self.Step` (+ (`self.Step`) 500))
      (else
        (for _index_2 (range (- _returnvalue 500) (+ _returnvalue 1))
          (switch `int` `color selection`
            (:`Default`
              (bind _outinstancetransform_2 (`InstancedStaticMeshComponent.GetInstanceTransform` buffer _index_2 false))
              (`self.Spawn Yellow Dot` (.location _outinstancetransform_2) (.rotation _outinstancetransform_2) :!label _label_2))
            (:`0`
              (goto _label_2))
            (:`1`
              (`self.Spawn Green Dot` (.location _outinstancetransform_2) (.rotation _outinstancetransform_2)))
            (:`2`
              (`self.Spawn Blue Dot` (.location _outinstancetransform_2) (.rotation _outinstancetransform_2)))
            (:`3`
              (`self.Spawn Red Dot` (.location _outinstancetransform_2) (.rotation _outinstancetransform_2)))))
        (set `self.Step` (+ (`self.Step`) 500))))))

(fn `UserConstructionScript`)