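; Lidar scanner gun that paints colored dots on surfaces it hits.
; Timed loops fire random line traces, either in an adjustable-spread cone or as a top-to-bottom wide scan with a recharge delay.
; FireLaser sends hits to BP_LaserPointSceneInstance as instanced points colored by actor class, and speeds up enemies it hits.
; Hit locations feed a Niagara array for beam effects, thinned during wide scans to save frames.
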(event `self.ReceiveBeginPlay`
  ;[1 1 1] Get laser Point Blueprint In scene
  (bind _outactors (`GameplayStatics.GetAllActorsOfClass` "/Game/Scanner_Gun/Blueprints/BP_LaserPointSceneInstance.BP_LaserPointSceneInstance_C"))
  (set `self.Laser Scene` (`|GetArrayItem` _outactors)))

(event `Stop Fire`
  (bind _lasergunsound (`self.LaserGunSound`))
  ;[1 1 1] Fire
  (if (not (`self.largeScan?`))
    (`KismetSystemLibrary.K2_ClearAndInvalidateTimerHandle` (stale `Fire` _returnvalue))
    (`/Engine/EditorBlueprintResources/StandardMacros.IsValid` _lasergunsound
      (:`Is Valid`
        (`AudioComponent.Stop` _lasergunsound))
      (:`Is Not Valid`
        _))
    (set `self.fire?` false)
    (`NiagaraDataInterfaceArrayFunctionLibrary.SetNiagaraArrayVector` (`self.FXS_Laser`) "LaserVectorArray" (`self.LaserVectors`))
    (`ActorComponent.Deactivate` (`self.FXS_Laser`))))

(event `Debug On`
  ;[1 0.03075 0.06059] debug
  (bind _returnvalue (`KismetSystemLibrary.K2_SetTimerDelegate` (delegate `debug`) 1.0 true))
  (`SceneComponent.SetHiddenInGame` (`self.Arrow`) false false))

(event `Fire`
  ;[1 1 1] Fire
  (if (not (`self.largeScan?`))
    (set `self.fire?` true)
    (bind _returnvalue (`KismetSystemLibrary.K2_SetTimerDelegate` (delegate `Fire Loop`) (`self.Laser Interval`) true))
    (`self.createLaserGunSound`)))

(event `debug`
  ;[1 0.03075 0.06059] debug
  (`KismetSystemLibrary.PrintString` (`KismetStringLibrary.Conv_IntToString` (`self.Count`))))

(event `Fire Loop`
  (bind _spread (`self.Spread`))
  (bind _arrow (`self.Arrow`))
  (bind _lasergunsound (`self.LaserGunSound`))
  (bind _returnvalue (`SceneComponent.K2_GetComponentLocation` _arrow))
  ;[1 1 1] Fire
  (`KismetArrayLibrary.Array_Clear` (`self.LaserVectors`))
  (for _ (range (+ (`self.ShotNumber`) 1))
    (`/Engine/EditorBlueprintResources/StandardMacros.IsValid` _lasergunsound
      (:`Is Valid`
        (`AudioComponent.SetFloatParameter` _lasergunsound "laserPitch" (/ _spread 10.0)))
      (:`Is Not Valid`
        _))
    (`self.Fire Laser` _returnvalue (+ _returnvalue (* (`KismetMathLibrary.RandomUnitVectorInConeInDegrees` (`SceneComponent.GetForwardVector` _arrow) _spread) 1500000)))
    ;;[1 0.03075 0.06059] Debug Only
    (`/Engine/EditorBlueprintResources/StandardMacros.IncrementInt` (`self.Count`)
      (:`  `
        ;;[1 0.7665 0.09399] avoid spamming the sound too much and saturating it
        (if (`KismetMathLibrary.RandomBoolWithWeight` 0.1)
          (`GameplayStatics.PlaySoundAtLocation` "/Game/Scanner_Gun/Sounds/SC_laserSound1.SC_laserSound1" _returnvalue (struct) 0.1 0.5 0.0 null null null null)))))
  (`NiagaraDataInterfaceArrayFunctionLibrary.SetNiagaraArrayVector` (`self.FXS_Laser`) "LaserVectorArray" (`self.LaserVectors`))
  (`ActorComponent.Activate` (`self.FXS_Laser`) true))

(event `Debug Off`
  ;[1 0.03075 0.06059] debug
  (`KismetSystemLibrary.K2_ClearAndInvalidateTimerHandle` (stale `Debug On` _returnvalue))
  (`SceneComponent.SetHiddenInGame` (`self.Arrow`) true false))

(event `Increase Spread`
  ;[1 1 1] Fire
  ;;[1 1 1] Increase/Decrease Spread Ring
  (set `self.Spread` (`KismetMathLibrary.FClamp` (+ (`self.Spread`) 2.0) (`self.Min Spread`) (`self.Max Spread`))))

(event `Decrease Spread`
  ;[1 1 1] Fire
  ;;[1 1 1] Increase/Decrease Spread Ring
  (set `self.Spread` (`KismetMathLibrary.FClamp` (- (`self.Spread`) 2.0) (`self.Min Spread`) (`self.Max Spread`))))

(event `Screen Scan`
  (bind _arrow (`self.Arrow`))
  (bind (_relativerotation_roll _relativerotation_pitch _relativerotation_yaw) (`KismetMathLibrary.BreakRotator` (`SceneComponent.RelativeRotation` _arrow)))
  ;[1 1 1] Laser Wave
  (`/Engine/EditorBlueprintResources/StandardMacros.Gate` false :!label _label
    (:`Exit`
      (if (not (not (`self.fire?`)))
        (`self.Stop Fire`))
      (set `self.largeScan?` true)
      (`self.createLaserGunSound`)
      (set `self.Loop` 0)
      (set `self.Z` (+ (.z (`SceneComponent.GetForwardVector` _arrow)) 0.6))
      (`SceneComponent.K2_SetRelativeRotation` (`self.Arrow`) (`KismetMathLibrary.MakeRotator` _relativerotation_roll 70.0 _relativerotation_yaw) false false)
      (bind _returnvalue (`KismetSystemLibrary.K2_SetTimerDelegate` (delegate `CustomEvent`) (+ (`self.Laser Interval`) 0.03) true))
      (goto _label :!via `Close`))))

(event `CustomEvent`
  (bind _lasergunsound (`self.LaserGunSound`))
  (bind _loop (`self.Loop`))
  (bind _arrow (`self.Arrow`))
  (bind _returnvalue (`SceneComponent.K2_GetComponentLocation` (`self.Arrow`)))
  (bind (_relativerotation_roll _relativerotation_pitch _relativerotation_yaw) (`KismetMathLibrary.BreakRotator` (`SceneComponent.RelativeRotation` _arrow)))
  (bind _x (.x (`KismetMathLibrary.RandomUnitVectorInEllipticalConeInDegrees` (`KismetMathLibrary.MakeVector` (.x (`SceneComponent.GetForwardVector` _arrow)) (.y (`SceneComponent.GetForwardVector` _arrow)) (`self.Z`)) 80.0 10.0)))
  (bind _z (.z (`KismetMathLibrary.RandomUnitVectorInEllipticalConeInDegrees` (`KismetMathLibrary.MakeVector` (.x (`SceneComponent.GetForwardVector` _arrow)) (.y (`SceneComponent.GetForwardVector` _arrow)) (`self.Z`)) 80.0 10.0)))
  ;[1 1 1] Laser Wave
  (`KismetArrayLibrary.Array_Clear` (`self.LaserVectors`))
  (if (== _loop 75)
    ;;[1 1 1] When laser reach all the way down, reset arrow, stop sound, deactivate laser and stop timer
    (`ActorComponent.Deactivate` (`self.FXS_Laser`))
    (`SceneComponent.K2_SetRelativeRotation` (`self.Arrow`) (`KismetMathLibrary.MakeRotator` _relativerotation_roll 0.0 _relativerotation_yaw) false false)
    (`/Engine/EditorBlueprintResources/StandardMacros.IsValid` _lasergunsound
      (:`Is Valid`
        (`AudioComponent.Stop` _lasergunsound))
      (:`Is Not Valid`
        _))
    (`KismetSystemLibrary.K2_ClearAndInvalidateTimerHandle` (stale `Screen Scan` _returnvalue))
    (set `self.largeScan?` false)
    (`KismetSystemLibrary.Delay` 1.2)
    (`GameplayStatics.PlaySoundAtLocation` "/Game/NewAsset/SFX/CU_Recharge.CU_Recharge" (`SceneComponent.K2_GetComponentLocation` (`self.LidarGun`)) (struct) 0.3 1.0 0.0 null null null null)
    (`KismetSystemLibrary.Delay` 0.2)
    (goto _label :!via `Open`)
    (else
      (`SceneComponent.K2_SetRelativeRotation` (`self.Arrow`) (`KismetMathLibrary.MakeRotator` _relativerotation_roll (- _relativerotation_pitch 2.0) _relativerotation_yaw) false false)
      (`/Engine/EditorBlueprintResources/StandardMacros.IncrementInt` _loop
        (:`  `
          ;;[1 1 1] Decreasig Z value will bring up to down the linad scan
          (set `self.Z` (- (`self.Z`) 0.015))
          (for _ (range 301)
            ;;[1 0.03075 0.06059] Debug Only
            (`/Engine/EditorBlueprintResources/StandardMacros.IncrementInt` (`self.Count`)
              (:`  `
                (`self.Fire Laser` _returnvalue (+ _returnvalue (* (`KismetMathLibrary.VLerp` (`KismetMathLibrary.MakeVector` (`KismetMathLibrary.RandomFloatInRange` -1.1 1.0) (.y (`KismetMathLibrary.RandomUnitVectorInEllipticalConeInDegrees` (`KismetMathLibrary.MakeVector` (.x (`SceneComponent.GetForwardVector` _arrow)) (.y (`SceneComponent.GetForwardVector` _arrow)) (`self.Z`)) 80.0 10.0)) _z) (`KismetMathLibrary.MakeVector` _x (`KismetMathLibrary.RandomFloatInRange` -1.1 1.1) _z) (`KismetMathLibrary.Abs` _x)) 500000)) true)
                ;;[1 0.7665 0.09399] avoid spamming the sound too much and saturating it
                (if (`KismetMathLibrary.RandomBoolWithWeight` 0.005)
                  (`GameplayStatics.PlaySoundAtLocation` "/Game/Scanner_Gun/Sounds/SC_laserSound1.SC_laserSound1" _returnvalue (struct) 0.1 0.5 0.0 null null null null)))))
          (`NiagaraDataInterfaceArrayFunctionLibrary.SetNiagaraArrayVector` (`self.FXS_Laser`) "LaserVectorArray" (`self.LaserVectors`))
          (`ActorComponent.Activate` (`self.FXS_Laser`) true))))))

(fn `Fire Laser`
  (params (Start :type "Vector Structure") (End :type "Vector Structure") (LimitParticle :type Boolean))
  (locals (NewLocalVar :type "Float (single-precision)" :default 0.0))
  (bind _laser_scene (`self.Laser Scene`))
  (bind _outhit (`KismetSystemLibrary.LineTraceSingle` Start End "TraceTypeQuery2" false (`|MakeArray` (`self.Player Ref`) (`self.Player Ref2`) :!type "Actor Object Reference") "None" true (struct :`R` 1.0 :`A` 1.0) (struct :`G` 1.0 :`A` 1.0) 2.0))
  (if (`GameplayStatics.BreakHitResult` _outhit)
    (`/Engine/EditorBlueprintResources/StandardMacros.IsValid` (`.HitComponent` (`GameplayStatics.BreakHitResult` _outhit))
      (:`Is Valid`
        (`/Engine/EditorBlueprintResources/StandardMacros.IsValid` (`self.Laser Scene`)
          (:`Is Valid`
            ;[1 1 1] If you want to limite the particle spawn and get more fps
            (if LimitParticle
              (if (`KismetMathLibrary.RandomBoolWithWeight` 0.005)
                (`KismetArrayLibrary.Array_Add` (`self.LaserVectors`) (`.Location` (`GameplayStatics.BreakHitResult` _outhit)) :!label _label))
              (else
                (goto _label)))
            (cast `/Game/Scanner_Gun/Blueprints/BP_Door` (`.HitActor` (`GameplayStatics.BreakHitResult` _outhit))
              (:`then`
                (bind _returnvalue (`KismetMathLibrary.Conv_VectorToRotator` (`.Normal` (`GameplayStatics.BreakHitResult` _outhit))))
                ;[0.1275 1 0.1756] Dot Color add to Hierarchical Instanced Static Mesh
                (`/Game/Scanner_Gun/Blueprints/BP_LaserPointSceneInstance.SpawnBufferGreenPoint` _laser_scene (`.Location` (`GameplayStatics.BreakHitResult` _outhit)) _returnvalue))
              (:`CastFailed`
                (cast `/Game/NewAsset/Objects/BP_Gate` (`.HitActor` (`GameplayStatics.BreakHitResult` _outhit))
                  (:`then`
                    (`/Game/Scanner_Gun/Blueprints/BP_LaserPointSceneInstance.SpawnBufferBluePoint` _laser_scene (`.Location` (`GameplayStatics.BreakHitResult` _outhit)) _returnvalue))
                  (:`CastFailed`
                    (cast `/Game/NewAsset/BP_Stalker` (`.HitActor` (`GameplayStatics.BreakHitResult` _outhit))
                      (:`then`
                        (`/Game/Scanner_Gun/Blueprints/BP_LaserPointSceneInstance.SpawnBufferBluePoint` _laser_scene (`.Location` (`GameplayStatics.BreakHitResult` _outhit)) _returnvalue))
                      (:`CastFailed`
                        (cast `/Game/NewAsset/Objects/BP_Buttoms` (`.HitActor` (`GameplayStatics.BreakHitResult` _outhit))
                          (:`then`
                            (`/Game/Scanner_Gun/Blueprints/BP_LaserPointSceneInstance.SpawnBufferGreenPoint` _laser_scene (`.Location` (`GameplayStatics.BreakHitResult` _outhit)) _returnvalue))
                          (:`CastFailed`
                            (cast `/Game/NewAsset/Objects/BP_Buttoms1` (`.HitActor` (`GameplayStatics.BreakHitResult` _outhit))
                              (:`then`
                                (`/Game/Scanner_Gun/Blueprints/BP_LaserPointSceneInstance.SpawnBufferGreenPoint` _laser_scene (`.Location` (`GameplayStatics.BreakHitResult` _outhit)) _returnvalue))
                              (:`CastFailed`
                                (cast `/Game/Scanner_Gun/Blueprints/props/BP_Props` (`.HitActor` (`GameplayStatics.BreakHitResult` _outhit))
                                  (:`then`
                                    (`/Game/Scanner_Gun/Blueprints/BP_LaserPointSceneInstance.SpawnBufferBluePoint` _laser_scene (`.Location` (`GameplayStatics.BreakHitResult` _outhit)) _returnvalue))
                                  (:`CastFailed`
                                    (bind _asbp_enemy (cast `/Game/Scanner_Gun/Blueprints/BP_Enemy` (`.HitActor` (`GameplayStatics.BreakHitResult` _outhit)))
                                      (:`then`
                                        (`/Game/Scanner_Gun/Blueprints/BP_LaserPointSceneInstance.SpawnBufferRedPoint` _laser_scene (`.Location` (`GameplayStatics.BreakHitResult` _outhit)) _returnvalue)
                                        (`/Game/Scanner_Gun/Blueprints/BP_Enemy.IncreaseSpeed` _asbp_enemy))
                                      (:`CastFailed`
                                        (cast `/Game/NewAsset/Objects/BP_MovingWall` (`.HitActor` (`GameplayStatics.BreakHitResult` _outhit))
                                          (:`then`
                                            (`/Game/Scanner_Gun/Blueprints/BP_LaserPointSceneInstance.SpawnBufferBluePoint` _laser_scene (`.Location` (`GameplayStatics.BreakHitResult` _outhit)) _returnvalue))
                                          (:`CastFailed`
                                            (`/Game/Scanner_Gun/Blueprints/BP_LaserPointSceneInstance.SpawnBufferYellowPoint` _laser_scene (`.Location` (`GameplayStatics.BreakHitResult` _outhit)) _returnvalue))))))))))))))))))
          (:`Is Not Valid`
            (`KismetSystemLibrary.PrintString` "BP_LaserPointSceneInstance Neede to be added in scene")))))))

(fn `UserConstructionScript`)