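; BP_Buttoms1 is a one-shot stone button that reports to BP_MovingWall when pressed.
; ButtomPress plays a sound, lets pawns pass through its cube, sets Press and calls CollectButtons on the wall found by class.
; It then briefly shows the coffin-door dialogue widget created at BeginPlay and destroys itself.
; The box overlap events are empty; the Interact prompt logic is disconnected and never runs.
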(event `self.ReceiveBeginPlay`
  (bind _returnvalue (`|CreateWidget` "/Game/Scanner_Gun/widget/dialogue_Stuff/12W_coffinDoorOpen.12W_coffinDoorOpen_C"))
  (set `self.coffinDoorDialogue` _returnvalue))

(event `ButtomPress`
  (bind _coffindoordialogue (`self.coffinDoorDialogue`))
  (`GameplayStatics.PlaySound2D` "/Game/Scanner_Gun/Sounds/stone_button_press.stone_button_press" 1.0 1.0 0.0 null null)
  (`PrimitiveComponent.SetCollisionResponseToChannel` (`self.Cube`) "ECC_Pawn" "ECR_Ignore")
  (set `self.Press?` true)
  (bind _returnvalue (`GameplayStatics.GetActorOfClass` "/Game/NewAsset/Objects/BP_MovingWall.BP_MovingWall_C"))
  (`/Game/NewAsset/Objects/BP_MovingWall.CollectButtons` _returnvalue)
  (`KismetSystemLibrary.Delay` 2.0)
  (`UserWidget.AddToViewport` _coffindoordialogue 0)
  (`KismetSystemLibrary.Delay` 4.0)
  (`Widget.RemoveFromParent` _coffindoordialogue)
  (`self.K2_DestroyActor`))

(event `self.Box.OnComponentBeginOverlap`
  (params (OverlappedComponent :type "PrimitiveComponent Object Reference") (OtherActor :type "Actor Object Reference") (OtherComp :type "PrimitiveComponent Object Reference") (OtherBodyIndex :type Integer) (bFromSweep :type Boolean) (SweepResult :type "HitResult Structure (by ref)")))

(event `self.Box.OnComponentEndOverlap`
  (params (OverlappedComponent :type "PrimitiveComponent Object Reference") (OtherActor :type "Actor Object Reference") (OtherComp :type "PrimitiveComponent Object Reference") (OtherBodyIndex :type Integer)))

(fn `ButtomPressConfirm`)

(fn `UserConstructionScript`)