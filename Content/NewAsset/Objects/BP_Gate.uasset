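; Gate actor that opens once enough buttons have been collected.
; CollectButtoms increments a counter and, on reaching the maximum, fires OpenGate through a DoOnce so it triggers only one time.
; OpenGate plays a timeline whose GateLocationZ track drives a Lerp into the Gate's world Z location, though both Lerp endpoints are zero, so the resulting Z stays at zero.
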(event `OpenGate`
  (bind (_direction _gate_location_z) (`Timeline|Open Gate`)
    (:`Update`
      (`SceneComponent.K2_SetWorldLocation` (`self.Gate`) (`KismetMathLibrary.MakeVector` 0.0 0.0 (`KismetMathLibrary.Lerp` 0.0 0.0 _gate_location_z)) false false))))

(event `Collect Buttoms`
  (`/Engine/EditorBlueprintResources/StandardMacros.IncrementInt` (`self.CurButtomsCollected`)
    (:`  `
      (if (>= (`self.CurButtomsCollected`) (`self.MaxButtomsCollected`))
        (`/Engine/EditorBlueprintResources/StandardMacros.DoOnce` false
          (:`Completed`
            (`self.OpenGate`)))))))

(fn `UserConstructionScript`)