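; BP_Buttoms is a one-shot button that reports its press to the gate.
; ButtomPress lets pawns pass through its Cube, marks it pressed and calls CollectButtoms on the BP_Gate found in the level.
; After a delay it briefly shows the door-opening widget created at BeginPlay, then destroys itself.
; The Box overlap events are empty, and the Interact prompt logic is disconnected.
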(event `self.ReceiveBeginPlay`
  (bind _returnvalue (`|CreateWidget` "/Game/Scanner_Gun/widget/dialogue_Stuff/02W_startingDoorOpen.02W_startingDoorOpen_C"))
  (set `self.doorOpened` _returnvalue))

(event `ButtomPress`
  (bind _dooropened (`self.doorOpened`))
  (`PrimitiveComponent.SetCollisionResponseToChannel` (`self.Cube`) "ECC_Pawn" "ECR_Ignore")
  (set `self.Press?` true)
  (`/Engine/EditorBlueprintResources/StandardMacros.DoOnce` false
    (:`Completed`
      (bind _returnvalue (`GameplayStatics.GetActorOfClass` "/Game/NewAsset/Objects/BP_Gate.BP_Gate_C"))
      (`/Game/NewAsset/Objects/BP_Gate.Collect Buttoms` _returnvalue)
      (`KismetSystemLibrary.Delay` 2.0)
      (`UserWidget.AddToViewport` _dooropened 0)
      (`KismetSystemLibrary.Delay` 4.0)
      (`Widget.RemoveFromParent` _dooropened)
      (`self.K2_DestroyActor`)
      (`KismetSystemLibrary.PrintString` "Hello"))))

(event `self.Box.OnComponentBeginOverlap`
  (params (OverlappedComponent :type "PrimitiveComponent Object Reference") (OtherActor :type "Actor Object Reference") (OtherComp :type "PrimitiveComponent Object Reference") (OtherBodyIndex :type Integer) (bFromSweep :type Boolean) (SweepResult :type "HitResult Structure (by ref)")))

(event `self.Box.OnComponentEndOverlap`
  (params (OverlappedComponent :type "PrimitiveComponent Object Reference") (OtherActor :type "Actor Object Reference") (OtherComp :type "PrimitiveComponent Object Reference") (OtherBodyIndex :type Integer)))

(fn `ButtomPressConfirm`)

(fn `UserConstructionScript`)