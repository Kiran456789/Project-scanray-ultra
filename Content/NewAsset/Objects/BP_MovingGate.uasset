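; BP_MovingGate is a stone gate actor that opens after enough button presses.
; Each CountButtons call increments a counter, and reaching MaxButtonPress fires OpenGate once through a DoOnce.
; OpenGate plays a 2D sliding sound and runs the Open timeline, which sets the Cube's world Z from a Lerp whose endpoints are both zero in the graph.
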(event `OpenGate`
  (`GameplayStatics.PlaySound2D` "/Game/SFXnAudios/SFX/Environmental/stoneDoorSlide_-Trimmed.stoneDoorSlide_-Trimmed" 1.0 1.0 0.0 null null)
  (bind (_direction _newtrack_0) (`Timeline|Open`)
    (:`Update`
      (`SceneComponent.K2_SetWorldLocation` (`self.Cube`) (`KismetMathLibrary.MakeVector` 0.0 0.0 (`KismetMathLibrary.Lerp` 0.0 0.0 _newtrack_0)) false false))))

(event `CountButtons`
  (`/Engine/EditorBlueprintResources/StandardMacros.IncrementInt` (`self.CurrentButtonPress`)
    (:`  `
      (if (>= (`self.CurrentButtonPress`) (`self.MaxButtonPress`))
        (`/Engine/EditorBlueprintResources/StandardMacros.DoOnce` false
          (:`Completed`
            (`self.OpenGate`)))))))

(fn `UserConstructionScript`)