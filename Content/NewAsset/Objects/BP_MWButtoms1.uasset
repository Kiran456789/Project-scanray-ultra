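; BP_MWButtoms1 is a one-shot button that counts toward opening or driving BP_MovingWall.
; ButtomPress disables the cube's Pawn collision, sets Press, calls CollectButtons on the first BP_MovingWall found, then destroys the actor.
; The Box overlap events are empty: the Interact prompt widget logic for characters is disconnected and never runs.
; ButtomPressConfirm is an empty stub.
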(event `ButtomPress`
  (`PrimitiveComponent.SetCollisionResponseToChannel` (`self.Cube`) "ECC_Pawn" "ECR_Ignore")
  (set `self.Press?` true)
  (bind _returnvalue (`GameplayStatics.GetActorOfClass` "/Game/NewAsset/Objects/BP_MovingWall.BP_MovingWall_C"))
  (`/Game/NewAsset/Objects/BP_MovingWall.CollectButtons` _returnvalue)
  (`self.K2_DestroyActor`))

(event `self.Box.OnComponentBeginOverlap`
  (params (OverlappedComponent :type "PrimitiveComponent Object Reference") (OtherActor :type "Actor Object Reference") (OtherComp :type "PrimitiveComponent Object Reference") (OtherBodyIndex :type Integer) (bFromSweep :type Boolean) (SweepResult :type "HitResult Structure (by ref)")))

(event `self.Box.OnComponentEndOverlap`
  (params (OverlappedComponent :type "PrimitiveComponent Object Reference") (OtherActor :type "Actor Object Reference") (OtherComp :type "PrimitiveComponent Object Reference") (OtherBodyIndex :type Integer)))

(fn `ButtomPressConfirm`)

(fn `UserConstructionScript`)