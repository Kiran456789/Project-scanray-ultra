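; BP_MovingWall is a wall actor that clears once enough buttons have been collected.
; CollectButtons increments a counter and, when it reaches the maximum, calls OpenMovingWall once through a DoOnce.
; OpenMovingWall plays a timeline whose update destroys the actor, so the wall disappears without moving.
; An unconnected SetWorldLocation node with a Z lerp, noted as the intended movement, never runs.
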(event `OpenMovingWall`
  (`Timeline|Timeline`
    (:`Update`
      (`self.K2_DestroyActor`))))

(event `CollectButtons`
  (`/Engine/EditorBlueprintResources/StandardMacros.IncrementInt` (`self.Cur Buttoms Collected`)
    (:`  `
      (if (>= (`self.Cur Buttoms Collected`) (`self.Max Buttoms Collected`))
        (`/Engine/EditorBlueprintResources/StandardMacros.DoOnce` false
          (:`Completed`
            (`self.OpenMovingWall`)))))))

(fn `UserConstructionScript`)