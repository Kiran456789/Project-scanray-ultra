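; BP_TempSpawner is a trigger actor that temporarily spawns a Stalker enemy when the player enters its box.
; BeginPlay caches the player's BP_ThirdPersonCharacter, and the box overlap checks against it, gated by a DoOnce so it fires only once.
; SpawnTempAI spawns BP_Stalker with BT_Stalker at the Billboard's location, then destroys that enemy, not the spawner, after 12 seconds.
; The StatueSpawn event plays at that location on both spawn and removal.
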(event `self.ReceiveBeginPlay`
  ;[1 1 1] spawns enemy and deletes itself atfer 12 seconds
  (bind _asbp_third_person_character (cast `/Game/Scanner_Gun/Blueprints/BP_ThirdPersonCharacter` (`GameplayStatics.GetPlayerCharacter` 0)))
  (set `self.As BP Third Person Character` _asbp_third_person_character))

(event `self.Box.OnComponentBeginOverlap`
  (params (OverlappedComponent :type "PrimitiveComponent Object Reference") (OtherActor :type "Actor Object Reference") (OtherComp :type "PrimitiveComponent Object Reference") (OtherBodyIndex :type Integer) (bFromSweep :type Boolean) (SweepResult :type "HitResult Structure (by ref)"))
  ;[1 1 1] spawns enemy and deletes itself atfer 12 seconds
  (if (== OtherActor (`self.As BP Third Person Character`))
    (`/Engine/EditorBlueprintResources/StandardMacros.DoOnce` false
      (:`Completed`
        (`self.Spawn Temp AI`)))))

(event `Spawn Temp AI`
  (bind _returnvalue (`SceneComponent.K2_GetComponentLocation` (`self.Billboard`)))
  (bind _returnvalue_2 (`KismetMathLibrary.Conv_VectorToTransform` _returnvalue))
  ;[1 1 1] spawns enemy and deletes itself atfer 12 seconds
  (`FMODBlueprintStatics.PlayEventAtLocation` "/Game/FMOD/Events/statueSpawn.statueSpawn" _returnvalue_2)
  (bind _returnvalue_3 (`AIBlueprintHelperLibrary.SpawnAIFromClass` "/Game/NewAsset/EnemyRelated/BP_Stalker.BP_Stalker_C" "/Game/NewAsset/EnemyRelated/BT_Stalker.BT_Stalker" _returnvalue (struct :`Yaw` 180.0) false null))
  (`KismetSystemLibrary.Delay` 12.0)
  (`self.K2_DestroyActor` _returnvalue_3)
  (`FMODBlueprintStatics.PlayEventAtLocation` "/Game/FMOD/Events/statueSpawn.statueSpawn" _returnvalue_2))

(fn `UserConstructionScript`)