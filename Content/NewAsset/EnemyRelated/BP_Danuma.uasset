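; BP_Danuma is an enemy-related hazard pairing a SpotLight with a Box that deals 1000 damage to the third-person character on hit.
; SpotLight activation activates the Box, then switches the light off after a random delay bounded by Duration and a fixed maximum.
; SpotLight deactivation deactivates the Box in turn; nothing in this Blueprint turns the light back on.
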(event `self.Box.OnComponentHit`
  (params (HitComponent :type "PrimitiveComponent Object Reference") (OtherActor :type "Actor Object Reference") (OtherComp :type "PrimitiveComponent Object Reference") (NormalImpulse :type "Vector Structure") (Hit :type "HitResult Structure (by ref)"))
  (bind _asbp_third_person_character (cast `/Game/Scanner_Gun/Blueprints/BP_ThirdPersonCharacter` OtherActor))
  (`GameplayStatics.ApplyDamage` _asbp_third_person_character 1000.0))

(event `self.SpotLight.OnComponentActivated`
  (params (Component :type "ActorComponent Object Reference") (bReset :type Boolean))
  (`ActorComponent.Activate` (`self.Box`) false)
  (`KismetSystemLibrary.Delay` (`KismetMathLibrary.RandomFloatInRange` (`self.Duration`) 10.0))
  (`ActorComponent.Deactivate` (`self.SpotLight`)))

(event `self.SpotLight.OnComponentDeactivated`
  (params (Component :type "ActorComponent Object Reference"))
  (`ActorComponent.Deactivate` (`self.Box`)))

(fn `UserConstructionScript`)