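; BP_Grenade is a throwable projectile that pushes physics objects and makes a sound where it hits.
; On BeginPlay its two sphere components ignore the owner when moving.
; Each Hit applies a velocity-scaled impulse to simulating components and spawns an A_Sound actor with a set range, without destroying the grenade.
; Unconnected leftover nodes hold destroy, noise-report and BP_Fire spawn logic that never runs.
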(event `self.ReceiveBeginPlay`
  (`PrimitiveComponent.IgnoreActorWhenMoving` (`self.Sphere`) (`self.GetOwner`) true)
  (`PrimitiveComponent.IgnoreActorWhenMoving` (`self.Sphere1`) (`self.GetOwner`) true))

(event `self.ReceiveDestroyed`)

(event `self.ReceiveHit`
  (params (MyComp :type "PrimitiveComponent Object Reference") (Other :type "Actor Object Reference") (OtherComp :type "PrimitiveComponent Object Reference") (bSelfMoved :type Boolean) (HitLocation :type "Vector Structure") (HitNormal :type "Vector Structure") (NormalImpulse :type "Vector Structure") (Hit :type "HitResult Structure (by ref)"))
  (bind _returnvalue (`self.K2_GetActorLocation`))
  (if (`SceneComponent.IsSimulatingPhysics` OtherComp "None")
    (`PrimitiveComponent.AddImpulseAtLocation` OtherComp (* (`self.GetVelocity`) 10.0) _returnvalue "None"))
  (`|SpawnActorFromClass` "/Game/NewAsset/Throwable/SoundGen/A_Sound.A_Sound_C" (`KismetMathLibrary.MakeTransform` _returnvalue) "Undefined" "MultiplyWithRoot" null (struct :`R` 1.0 :`G` 1.0 :`B` 1.0 :`A` 1.0) 2500.0 0.0 null))

(fn `UserConstructionScript`)