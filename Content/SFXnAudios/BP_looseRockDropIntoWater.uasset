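; Trigger actor that stages a loose rock falling into water when the player character enters its RockDropTrigger volume.
; The first overlap by BP_ThirdPersonCharacter runs a one-shot timed sequence of 2D sound events: the rock drop, then the water splash.
; It then shows the pillar-collapsing dialogue widget, created at BeginPlay, for a few seconds before removing it from the screen.
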(event `self.ReceiveBeginPlay`
  (bind _returnvalue (`|CreateWidget` "/Game/Scanner_Gun/widget/dialogue_Stuff/14W_pillarCollapsing.14W_pillarCollapsing_C"))
  (set `self.pillarCollapsingDialogue` _returnvalue))

(event `self.rockDropTrigger.OnComponentBeginOverlap`
  (params (OverlappedComponent :type "PrimitiveComponent Object Reference") (OtherActor :type "Actor Object Reference") (OtherComp :type "PrimitiveComponent Object Reference") (OtherBodyIndex :type Integer) (bFromSweep :type Boolean) (SweepResult :type "HitResult Structure (by ref)"))
  (bind _pillarcollapsingdialogue (`self.pillarCollapsingDialogue`))
  (cast `/Game/Scanner_Gun/Blueprints/BP_ThirdPersonCharacter` OtherActor)
  (`/Engine/EditorBlueprintResources/StandardMacros.DoOnce` false
    (:`Completed`
      (`FMODBlueprintStatics.PlayEvent2D` "/Game/FMOD/Events/Environment/LooseRockDrop.LooseRockDrop")
      (`KismetSystemLibrary.Delay` 1.5)
      (`FMODBlueprintStatics.PlayEvent2D` "/Game/FMOD/Events/Environment/StoneDropInWater.StoneDropInWater")
      (`KismetSystemLibrary.Delay` 1.0)
      (`UserWidget.AddToViewport` _pillarcollapsingdialogue 0)
      (`KismetSystemLibrary.Delay` 4.0)
      (`Widget.RemoveFromParent` _pillarcollapsingdialogue))))

(fn `UserConstructionScript`)