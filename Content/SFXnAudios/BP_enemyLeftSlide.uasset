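; BP_enemyLeftSlide is a one-shot scare trigger that plays enemy movement audio and a gasp reaction when the player character walks into it.
; It creates the gasp widget at BeginPlay, then waits for a third-person character to overlap EnemyCreepTrigger.
; The first overlap plays the movement sound event, then after a short delay plays dialogue static and shows the widget for a few seconds.
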(event `self.ReceiveBeginPlay`
  (bind _returnvalue (`|CreateWidget` "/Game/Scanner_Gun/widget/dialogue_Stuff/03W_soundScareGasp.03W_soundScareGasp_C"))
  (set `self.gaspingVoiceover` _returnvalue))

(event `self.enemyCreepTrigger.OnComponentBeginOverlap`
  (params (OverlappedComponent :type "PrimitiveComponent Object Reference") (OtherActor :type "Actor Object Reference") (OtherComp :type "PrimitiveComponent Object Reference") (OtherBodyIndex :type Integer) (bFromSweep :type Boolean) (SweepResult :type "HitResult Structure (by ref)"))
  (bind _gaspingvoiceover (`self.gaspingVoiceover`))
  (cast `/Game/Scanner_Gun/Blueprints/BP_ThirdPersonCharacter` OtherActor)
  (`/Engine/EditorBlueprintResources/StandardMacros.DoOnce` false
    (:`Completed`
      (`FMODBlueprintStatics.PlayEvent2D` "/Game/FMOD/Events/Movement/enemyMovement.enemyMovement")
      (`KismetSystemLibrary.Delay` 1.0)
      (`GameplayStatics.PlaySound2D` "/Game/SFXnAudios/SFX/staticForDialogue.staticForDialogue" 1.0 1.0 0.0 null null)
      (`UserWidget.AddToViewport` _gaspingvoiceover 0)
      (`KismetSystemLibrary.Delay` 4.0)
      (`Widget.RemoveFromParent` _gaspingvoiceover))))

(fn `UserConstructionScript`)